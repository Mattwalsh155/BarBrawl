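; Destructible pool actor made of eleven destructible components that shatter together when its Break event is called.
; Break applies identical damage and a strong impulse to each component in turn, all pushed along world +Y via the right vector of a zero rotation.
; Each hit location uses the component's relative location rather than its world position.
; Nothing in this Blueprint calls Break, and the construction script is empty.
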(event Custom|Break
  (bind _destructible1 (Variables|Default|GetDestructible1))
  (bind _destructible2 (Variables|Default|GetDestructible2))
  (bind _destructible3 (Variables|Default|GetDestructible3))
  (bind _destructible4 (Variables|Default|GetDestructible4))
  (bind _destructible5 (Variables|Default|GetDestructible5))
  (bind _destructible6 (Variables|Default|GetDestructible6))
  (bind _destructible7 (Variables|Default|GetDestructible7))
  (bind _destructible8 (Variables|Default|GetDestructible8))
  (bind _destructible9 (Variables|Default|GetDestructible9))
  (bind _destructible10 (Variables|Default|GetDestructible10))
  (bind _destructible (Variables|Default|GetDestructible))
  (Class|DestructibleComponent|ApplyDamage _destructible 5e+01 (Variables|/Script/Engine.SceneComponent|GetRelativeLocation _destructible) (Math|Vector|GetRightVector "0,0.000000, 0") 3e+03)
  (Class|DestructibleComponent|ApplyDamage _destructible1 5e+01 (Variables|/Script/Engine.SceneComponent|GetRelativeLocation _destructible1) (Math|Vector|GetRightVector "0.000000,0.000000,0.000000") 3e+03)
  (Class|DestructibleComponent|ApplyDamage _destructible2 5e+01 (Variables|/Script/Engine.SceneComponent|GetRelativeLocation _destructible2) (Math|Vector|GetRightVector "0, 0, 0") 3e+03)
  (Class|DestructibleComponent|ApplyDamage _destructible3 5e+01 (Variables|/Script/Engine.SceneComponent|GetRelativeLocation _destructible3) (Math|Vector|GetRightVector "0, 0, 0") 3e+03)
  (Class|DestructibleComponent|ApplyDamage _destructible4 5e+01 (Variables|/Script/Engine.SceneComponent|GetRelativeLocation _destructible4) (Math|Vector|GetRightVector "0, 0, 0") 3e+03)
  (Class|DestructibleComponent|ApplyDamage _destructible5 5e+01 (Variables|/Script/Engine.SceneComponent|GetRelativeLocation _destructible5) (Math|Vector|GetRightVector "0, 0, 0") 3e+03)
  (Class|DestructibleComponent|ApplyDamage _destructible6 5e+01 (Variables|/Script/Engine.SceneComponent|GetRelativeLocation _destructible6) (Math|Vector|GetRightVector "0, 0, 0") 3e+03)
  (Class|DestructibleComponent|ApplyDamage _destructible7 5e+01 (Variables|/Script/Engine.SceneComponent|GetRelativeLocation _destructible7) (Math|Vector|GetRightVector "0, 0, 0") 3e+03)
  (Class|DestructibleComponent|ApplyDamage _destructible8 5e+01 (Variables|/Script/Engine.SceneComponent|GetRelativeLocation _destructible8) (Math|Vector|GetRightVector "0, 0, 0") 3e+03)
  (Class|DestructibleComponent|ApplyDamage _destructible9 5e+01 (Variables|/Script/Engine.SceneComponent|GetRelativeLocation _destructible9) (Math|Vector|GetRightVector "0, 0, 0") 3e+03)
  (Class|DestructibleComponent|ApplyDamage _destructible10 5e+01 (Variables|/Script/Engine.SceneComponent|GetRelativeLocation _destructible10) (Math|Vector|GetRightVector "0, 0, 0") 3e+03))

(event EventBeginPlay)

(event Collision|EventActorBeginOverlap
  (params (OtherActor :type Actor%20Object%20Reference)))

(event EventTick
  (params (DeltaSeconds :type Float%20%28single-precision%29)))

(fn ConstructionScript)